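; BP_GridManager is an actor that defines a square-cell grid anchored at its location and draws it in the world.
; On BeginPlay it adds one slightly shrunken, slightly raised instance per cell to the Cells instanced mesh component.
; Helper functions convert between world positions and cell coordinates, returning cell centres, and test whether a cell is inside the bounds.
; ShowCell moves the Highlight component just above a given cell.
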(event `self.ReceiveBeginPlay`
  (for _index (range (`self.CellCountX`))
    (for _index_2 (range (`self.CellCountY`))
      (bind _position (`self.GridToWorld` (make `IntPoint` _index _index_2)))
      (`InstancedStaticMeshComponent.AddInstance` (`self.Cells`) (`KismetMathLibrary.MakeTransform` (+ _position (0.0 0.0 1.0)) (struct) (0.95 0.95 1.0)) true))))

(fn `GridToWorld`
  (params (Cell :type "IntPoint Structure"))
  (returns (Position :type "Vector Structure"))
  (bind (_x _y) (break `IntPoint` Cell))
  (bind _returnvalue (/ (`self.CellSize`) 2.0))
  (return (`KismetMathLibrary.MakeVector` (+ (* _x (`self.CellSize`)) (.x (`self.K2_GetActorLocation`)) _returnvalue) (+ (* _y (`self.CellSize`)) (.y (`self.K2_GetActorLocation`)) _returnvalue) (.z (`self.K2_GetActorLocation`)))))

(fn `IsInsideGrid`
  (params (Cell :type "IntPoint Structure"))
  (returns (Inside :type Boolean))
  (bind (_x _y) (break `IntPoint` Cell))
  (return (and (>= _x 0) (< _x (`self.CellCountX`)) (>= _y 0) (< _y (`self.CellCountY`)))))

(fn `ShowCell`
  (params (Cell :type "IntPoint Structure"))
  (bind _position (`self.GridToWorld` Cell))
  (`SceneComponent.K2_SetWorldLocation` (`self.Highlight`) (+ _position (0.0 0.0 2.0)) false false))

(fn `UserConstructionScript`)

(fn `WorldToGrid`
  (params (Position :type "Vector Structure"))
  (returns (Cell :type "IntPoint Structure"))
  (return (make `IntPoint` (`KismetMathLibrary.FFloor` (/ (- (.x Position) (.x (`self.K2_GetActorLocation`))) (`self.CellSize`))) (`KismetMathLibrary.FFloor` (/ (- (.y Position) (.y (`self.K2_GetActorLocation`))) (`self.CellSize`))))))