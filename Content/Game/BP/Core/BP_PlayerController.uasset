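; Player controller that tracks which grid cell is under the mouse cursor and shows it.
; On BeginPlay it adds the default Enhanced Input mapping context and caches the level's BP_GridManager.
; Each tick it traces under the cursor on the Visibility channel, converts the impact point to a grid cell, stores it as HoveredCell and tells the grid manager to show it.
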(event `self.ReceiveBeginPlay`
  (`EnhancedInputSubsystemInterface.AddMappingContext` (subsystem `EnhancedInputLocalPlayerSubsystem`) "/Game/Game/Input/IMC_Default.IMC_Default" 0 (struct))
  (bind _returnvalue (`GameplayStatics.GetActorOfClass` "/Game/Game/BP/Grid/BP_GridManager.BP_GridManager_C"))
  (set `self.GridManager` _returnvalue))

(event `self.ReceiveTick`
  (params (DeltaSeconds :type "Float (single-precision)"))
  (bind (_hitresult _returnvalue) (`self.GetHitResultUnderCursorByChannel` "TraceTypeQuery1"))
  (if _returnvalue
    (bind _cell (`/Game/Game/BP/Grid/BP_GridManager.WorldToGrid` (`self.GridManager`) (`.ImpactPoint` (`GameplayStatics.BreakHitResult` _hitresult))))
    (set `self.HoveredCell` _cell)
    (`/Game/Game/BP/Grid/BP_GridManager.ShowCell` (`self.GridManager`) (`self.HoveredCell`))))

(fn `UserConstructionScript`)